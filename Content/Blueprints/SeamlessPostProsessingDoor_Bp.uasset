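; Doorway actor that seamlessly switches the first-person camera's post-process look when the player walks through it.
; While the player overlaps PlayerDetection, Tick detects crossings using the camera's side of the door plane and a line-plane intersection from its last position.
; Each crossing toggles IsInverted, swapping the Entry material and camera post-process blendable.
; PreventPlaneClipping nudges the Entry mesh away from a nearby camera to avoid clipping.
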(event EventBeginPlay)

(event Collision|EventActorBeginOverlap
  (params (OtherActor :type Actor%20Object%20Reference)))

(event EventTick
  (params (DeltaSeconds :type Float%20%28single-precision%29))
  (if (Collision|IsOverlappingActor (Variables|Default|GetPlayerDetection) (Game|GetPlayerCharacter 0) :!class /Script/Engine.PrimitiveComponent)
    (CallFunction|PreventPlaneClipping)
    (bind _iscrossing1 (CallFunction|HasCrossedDoor))
    (if _iscrossing1
      (if (Variables|Default|GetIsInverted)
        (Variables|Default|SetIsInverted false)
        (Rendering|Material|SetMaterial (Variables|Default|GetEntry) 0 (Variables|Default|GetDoorMaterial))
        (Variables|/Script/Engine.CameraComponent|SetPostProcessSettings (Variables|/Script/SeamlessPostProcess.SeamlessPostProcessCharacter|GetFirstPersonCameraComponent (.AsBP%20First%20Person%20Character (Utilities|Casting|CastToBP_FirstPersonCharacter (Game|GetPlayerCharacter 0)))) (Utilities|Struct|MakePostProcessSettings (Utilities|Struct|MakeWeightedBlendables (Utilities|Array|MakeArray (Utilities|Struct|MakeWeightedBlendable 1.0 "/Game/Materials/SeemlessPostProcessing/Default_Shader_PPM.Default_Shader_PPM")))))
        (else
          (Variables|Default|SetIsInverted true)
          (Rendering|Material|SetMaterial (Variables|Default|GetEntry) 0 "/Game/Materials/SeemlessPostProcessing/Default_Shader.Default_Shader")
          (Variables|/Script/Engine.CameraComponent|SetPostProcessSettings (Variables|/Script/SeamlessPostProcess.SeamlessPostProcessCharacter|GetFirstPersonCameraComponent (.AsBP%20First%20Person%20Character (Utilities|Casting|CastToBP_FirstPersonCharacter (Game|GetPlayerCharacter 0)))) (Utilities|Struct|MakePostProcessSettings (Utilities|Struct|MakeWeightedBlendables (Utilities|Array|MakeArray (Utilities|Struct|MakeWeightedBlendable 1.0 (Variables|Default|GetPostProcessMaterial)))))))))
    (else
      (Variables|Default|SetbIsOverlaping false))))

(fn ConstructionScript
  (Rendering|Material|SetMaterial (Variables|Default|GetEntry) 0 (Variables|Default|GetDoorMaterial)))

(fn HasCrossedDoor
  (LocalVariables|SetbIsInfront (>= (Math|Vector|DotProduct (- (Transformation|GetWorldLocation (Variables|/Script/SeamlessPostProcess.SeamlessPostProcessCharacter|GetFirstPersonCameraComponent (.AsBP%20First%20Person%20Character (Utilities|Casting|CastToBP_FirstPersonCharacter (Game|GetPlayerCharacter 0))))) (Transformation|GetActorLocation)) (Math|Vector|GetForwardVector (Variables|Default|GetForwardDirection))) 0.0))
  (bind _output_get (LocalVariables|SetDoorPlane (Class|KismetMathLibrary|MakePlanefromPointandNormal (Transformation|GetActorLocation) (Math|Vector|GetForwardVector (Variables|Default|GetForwardDirection)))))
  (LocalVariables|SetIsIntersecting (.ReturnValue (Class|KismetMathLibrary|LinePlaneIntersection (Transformation|GetWorldLocation (Variables|/Script/SeamlessPostProcess.SeamlessPostProcessCharacter|GetFirstPersonCameraComponent (.AsBP%20First%20Person%20Character (Utilities|Casting|CastToBP_FirstPersonCharacter (Game|GetPlayerCharacter 0))))) (Variables|Default|GetLastPosition) _output_get)))
  (LocalVariables|SetIsCrossing (or (Math|Boolean|ANDBoolean (LocalVariables|GetIsIntersecting) (not (LocalVariables|GetbIsInfront)) (Variables|Default|GetLastInFront) (Variables|Default|GetbIsOverlaping)) (Math|Boolean|ANDBoolean (LocalVariables|GetIsIntersecting) (LocalVariables|GetbIsInfront) (not (Variables|Default|GetLastInFront)) (Variables|Default|GetbIsOverlaping))))
  (Variables|Default|SetLastInFront (LocalVariables|GetbIsInfront))
  (Variables|Default|SetLastPosition (Transformation|GetWorldLocation (Variables|/Script/SeamlessPostProcess.SeamlessPostProcessCharacter|GetFirstPersonCameraComponent (.AsBP%20First%20Person%20Character (Utilities|Casting|CastToBP_FirstPersonCharacter (Game|GetPlayerCharacter 0))))))
  (Variables|Default|SetbIsOverlaping true)
  (return (LocalVariables|GetIsCrossing)))

(fn PreventPlaneClipping
  (bind _returnvalue (Game|GetPlayerCharacter 0))
  (bind _returnvalue_2 (Transformation|GetActorLocation))
  (bind _forwarddirection (Variables|Default|GetForwardDirection))
  (bind _returnvalue_3 (Math|Vector|GetForwardVector _forwarddirection))
  (bind _asbp_first_person_character (Utilities|Casting|CastToBP_FirstPersonCharacter _returnvalue))
  (bind _firstpersoncameracomponent (Variables|/Script/SeamlessPostProcess.SeamlessPostProcessCharacter|GetFirstPersonCameraComponent _asbp_first_person_character))
  (bind _returnvalue_4 (Transformation|GetWorldLocation _firstpersoncameracomponent))
  (bind _returnvalue_5 (- _returnvalue_4 _returnvalue_2))
  (bind _returnvalue_6 (Math|Vector|DotProduct _returnvalue_3 _returnvalue_5))
  (if (and (>= _returnvalue_6 -3.0) (<= _returnvalue_6 0.0))
    ;[1 1 1] 如果玩家靠在門的Mesh上，稍微把他移後面一點，避免卡在玩家的視角中間
    (Transformation|SetRelativeLocation (Variables|Default|GetEntry) "2.000000,0.000000,100.000000" false false)
    (elif (and (>= _returnvalue_6 0.0) (<= _returnvalue_6 3.0))
      ;[1 1 1] 如果玩家靠在門的Mesh上，稍微把他移後面一點，避免卡在玩家的視角中間
      (Transformation|SetRelativeLocation (Variables|Default|GetEntry) "-2.000000,0.000000,100.000000" false false)
      (else
        (Transformation|SetRelativeLocation (Variables|Default|GetEntry) "-0.000000,0.000000,100.000000" false false)))))